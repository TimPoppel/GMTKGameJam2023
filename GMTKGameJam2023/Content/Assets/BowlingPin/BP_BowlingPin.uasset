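; Bowling pin actor that decides whether it has fallen when the bowling game mode signals a pin check.
; On BeginPlay it binds CheckPins to GM_Bowling, then stores its starting location after a short delay.
; CheckPins compares current height to the stored height within a tolerance: a matching pin has its Cube moved below the starting spot, otherwise the actor destroys itself.
; Delayed versions of both outcomes are present but unconnected.
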(event Custom|Check%20Pins
  (bind _pin_starting_location (Variables|Default|GetPin%20Starting%20Location))
  (if (Math|Float|NearlyEqual(Float) (.z (Transformation|GetWorldLocation (Variables|Default|GetScene))) (.z (Variables|Default|GetPin%20Starting%20Location)) 5.0)
    (Transformation|SetWorldLocation (Variables|Default|GetCube) (Math|Vector|MakeVector (.x _pin_starting_location) (.y _pin_starting_location) (- (.z _pin_starting_location) 5e+01)) false false)
    (else
      (Actor|DestroyActor))))

(event EventBeginPlay
  (bind _asgm_bowling (Utilities|Casting|CastToGM_Bowling (Game|GetGameMode)))
  (EventDispatchers|BindEventtoCheckPins _asgm_bowling (EventDispatchers|CreateEvent :!event Custom|Check%20Pins))
  (Utilities|FlowControl|Delay 0.2)
  (Variables|Default|SetPin%20Starting%20Location (Transformation|GetWorldLocation (Variables|Default|GetScene))))

(fn ConstructionScript)