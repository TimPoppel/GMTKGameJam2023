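; Bowling game mode that runs rounds of a timed shop-and-build phase followed by ball waves against pins, paying currency for pins left standing.
; Each round previews balls from the WaveManager table on random spawners, then launches two, or three in the final round.
; BallFinished starts a pin-settle timer per wave; wave-end events score knocked pins to the scoreboard.
; It also creates the default settings save and raises gates at round five.
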(event Custom|Start%20Building%20Phase
  ;[1 1 1] Building Phase
  (Default|ToggleVisibility (Variables|Default|GetBuildZoneRef) true)
  (if (== (Variables|WaveSystem|GetRoundCounter) 5)
    (bind _outactors (Actor|GetAllActorsOfClass "/Game/Blueprints/BP_Gates.BP_Gates_C"))
    (for _array_element _outactors
      (Default|PutUpGates _array_element)))
  (Variables|WaveSystem|SetWaveCounter 0)
  (Default|CallStartBuilding)
  (if (not (== (Variables|WaveSystem|GetRoundCounter) (Variables|WaveSystem|GetMaxRounds)))
    _
    (else
      (Variables|Default|SetWave10 true)))
  (Variables|/Game/Blueprints/Player/BP_PlayerPawn.BP_PlayerPawn_C|SetBuildingPhaseEnabled (Variables|Default|GetPlayerRef) true)
  (Widget|SetVisibility (Variables|Default|GetShopRef) "Visible")
  (CallFunction|PreviewBallSpawn (Math|Integer|SelectInt 3 2 (>= (Variables|WaveSystem|GetRoundCounter) 10)))
  (Utilities|FlowControl|Delay (Variables|Default|GetPlayerBuildTime))
  (CallFunction|WaveStart)
  (Widget|SetVisibility (Variables|Default|GetShopRef) "Collapsed")
  (Default|ToggleVisibility (Variables|Default|GetBuildZoneRef) false)
  (Default|ToggleVisibility (Variables|Default|GetPlayerRef) false))

(event Custom|Wave%20Start
  ;[1 1 1] Wave Start
  (Default|CallSpawnNewPins)
  (Math|Integer|IncrementInt (Variables|WaveSystem|GetWaveCounter)
    (:%20%20
      (bind _asbp_player_pawn (Utilities|Casting|CastToBP_PlayerPawn (Game|Player|GetPlayerPawn 0)))
      (Variables|/Game/Blueprints/Player/BP_PlayerPawn.BP_PlayerPawn_C|SetBuildingPhaseEnabled _asbp_player_pawn false)
      (CallFunction|SpawnBowlingBall))))

(event Custom|Second%20Bowling%20Ball
  ;[1 1 1] Second Wave Start
  (Math|Integer|IncrementInt (Variables|WaveSystem|GetWaveCounter)
    (:%20%20
      (CallFunction|SpawnBowlingBall))))

(event Custom|Wave%20End
  ;[1 1 1] Wave End
  (bind _outactors (Actor|GetAllActorsOfClass "/Game/Assets/BowlingPin/BP_BowlingPin.BP_BowlingPin_C"))
  (Actor|DestroyActor _outactors)
  (if (< (Variables|WaveSystem|GetRoundCounter) (Variables|WaveSystem|GetMaxRounds))
    (Math|Integer|IncrementInt (Variables|WaveSystem|GetRoundCounter)
      (:%20%20
        (CallFunction|StartBuildingPhase)))))

(event Custom|Wave%2010%203rd%20Ball
  ;[1 1 1] Third Wave Start
  (Math|Integer|IncrementInt (Variables|WaveSystem|GetWaveCounter)
    (:%20%20
      (CallFunction|SpawnBowlingBall))))

(event Custom|End%20Wave%201
  ;[1 1 1] Wave 1 Ends
  (Default|CallCheckPins)
  (CallFunction|Calculate1stBallScore)
  (CallFunction|SecondBowlingBall))

(event Custom|End%20Wave%202
  ;[1 1 1] Wave 2 Ends
  (Default|CallCheckPins)
  (CallFunction|GivePlayerCurrency)
  (if (Variables|Default|GetWave10)
    (CallFunction|Calculate2ndBallScore)
    (CallFunction|Wave103rdBall)
    (else
      (CallFunction|Calculate2ndBallScore)
      (CallFunction|WaveEnd))))

(event Custom|End%20Wave%203
  ;[1 1 1] Wave 3 Ends
  (Default|CallCheckPins)
  (CallFunction|Calculate3rdBallScore)
  (CallFunction|WaveEnd))

(event EventBeginPlay
  (Variables|WaveSystem|SetRoundCounter 1)
  (CallFunction|GetPlayerRef)
  (bind _returnvalue (UserInterface|CreateWidget "/Game/Blueprints/Shop/WB_Shop.WB_Shop_C"))
  (bind _output_get (Variables|Default|SetShopRef _returnvalue))
  (UserInterface|Viewport|AddtoViewport _output_get 0)
  (bind _returnvalue_2 (Actor|GetActorOfClass "/Game/Blueprints/Player/BP_BuildZone.BP_BuildZone_C"))
  (Variables|Default|SetBuildZoneRef _returnvalue_2)
  (CallFunction|StartBuildingPhase)
  (Utilities|FlowControl|Sequence
    (:then_0
      (bind _returnvalue_3 (SaveGame|DoesSaveGameExist "Settings"))
      (if (not _returnvalue_3)
        (bind _returnvalue_4 (SaveGame|CreateSaveGameObject "/Game/UI/Settings/SG_Basic.SG_Basic_C"))
        (SaveGame|SaveGametoSlot _returnvalue_4 "Settings")))
    (:then_1
      (bind _returnvalue_5 (Game|GetCurrentLevelName true))
      (if (Utilities|Enum|Equal(Enum) _returnvalue_5 "LevelBowling")
        (bind _returnvalue_6 (UserInterface|CreateWidget "/Game/UI/WBP_ScoringTable.WBP_ScoringTable_C"))
        (UserInterface|Viewport|AddtoViewport _returnvalue_6 0)
        (Variables|Default|SetScoringTableReference _returnvalue_6)))))

(fn ConstructionScript)

(fn Calculate1stBallScore
  (Variables|PinScoring|SetScoreBall1 0)
  (Variables|PinScoring|SetScoreBall2 0)
  (Variables|PinScoring|SetPinsLeft 0)
  (Variables|PinScoring|SetPinsHitBall2 0)
  (Variables|PinScoring|SetPinsHitBall1 0)
  (bind _outactors (Actor|GetAllActorsOfClass "/Game/Assets/BowlingPin/BP_BowlingPin.BP_BowlingPin_C"))
  (bind _output_get (Variables|PinScoring|SetPinsLeft (Utilities|Array|Length _outactors)))
  (bind _output_get_2 (Variables|PinScoring|SetPinsHitBall1 (- (Variables|PinScoring|GetMaxPins) _output_get)))
  (Variables|PinScoring|SetScoreBall1 _output_get_2)
  (Default|UpdateScoreBoard (Variables|Default|GetScoringTableReference)))

(fn Calculate2ndBallScore
  (bind _outactors (Actor|GetAllActorsOfClass "/Game/Assets/BowlingPin/BP_BowlingPin.BP_BowlingPin_C"))
  (bind _output_get (Variables|PinScoring|SetPinsLeft (Utilities|Array|Length _outactors)))
  (bind _output_get_2 (Variables|PinScoring|SetPinsHitBall2 (- (- (Variables|PinScoring|GetMaxPins) (Variables|PinScoring|GetPinsHitBall1)) _output_get)))
  (Variables|PinScoring|SetScoreBall2 _output_get_2)
  (Default|UpdateScoreBoard (Variables|Default|GetScoringTableReference)))

(fn Calculate3rdBallScore
  (bind _outactors (Actor|GetAllActorsOfClass "/Game/Assets/BowlingPin/BP_BowlingPin.BP_BowlingPin_C"))
  (bind _output_get (Variables|PinScoring|SetPinsLeft (Utilities|Array|Length _outactors)))
  (bind _output_get_2 (Variables|PinScoring|SetPinsHitBall1 (- (- (Variables|PinScoring|GetMaxPins) (+ (Variables|PinScoring|GetPinsHitBall1) (Variables|PinScoring|GetPinsHitBall2))) _output_get)))
  (Variables|PinScoring|SetScoreBall3 _output_get_2)
  (Default|UpdateScoreBoard (Variables|Default|GetScoringTableReference)))

(fn GetPlayerRef
  (bind _asbp_player_pawn (Utilities|Casting|CastToBP_PlayerPawn (Game|Player|GetPlayerPawn 0)))
  (bind _output_get (Variables|Default|SetPlayerRef _asbp_player_pawn))
  (return _output_get))

(fn SpawnBowlingBall
  (bind _availablespawners (Variables|Default|GetAvailableSpawners))
  (bind _outactors (Actor|GetAllActorsOfClass "/Game/Blueprints/BP_BowlingBallSpawner.BP_BowlingBallSpawner_C"))
  (for _array_element _outactors
    (if (Variables|/Game/Blueprints/BP_BowlingBallSpawner.BP_BowlingBallSpawner_C|GetbPreview _array_element)
      (Utilities|Array|AddUnique _availablespawners _array_element)
      (else
        (Utilities|Array|RemoveItem _availablespawners _array_element))))
  (Default|SpawnBall (.OutItem (Utilities|Array|Random (Variables|Default|GetAvailableSpawners))))
  (return))

(fn BowlingBallFInished)

(fn BallFinished
  (bind _wavecounter (Variables|WaveSystem|GetWaveCounter))
  (if (== _wavecounter 1)
    (Utilities|Time|SetTimerbyEvent (EventDispatchers|CreateEvent :!event Custom|End%20Wave%201) (Variables|Default|GetTime%20for%20pins%20to%20drop))
    (return)
    (elif (== _wavecounter 2)
      (Utilities|Time|SetTimerbyEvent (EventDispatchers|CreateEvent :!event Custom|End%20Wave%202) (Variables|Default|GetTime%20for%20pins%20to%20drop))
      (return)
      (else
        (Utilities|Time|SetTimerbyEvent (EventDispatchers|CreateEvent :!event Custom|End%20Wave%203) (Variables|Default|GetTime%20for%20pins%20to%20drop))
        (return)))))

(fn FindWaveBall
  (params (BallNumber :type Integer))
  (bind _returnvalue (Utilities|GetDataTableRow (Variables|Default|GetWaveManager) (Utilities|String|StringToName (Utilities|String|Append "Round" (Utilities|String|ToString(Integer) (Variables|WaveSystem|GetRoundCounter)))))
    (:then
      (return (Utilities|Select :Index BallNumber :Option%200 (.Ball1 (Utilities|Struct|BreakF_Waves _returnvalue)) :Option%201 (.Ball2 (Utilities|Struct|BreakF_Waves _returnvalue)) :Option%202 (.Ball3 (Utilities|Struct|BreakF_Waves _returnvalue)))))))

(fn PreviewBallSpawn
  (params (PreviewAmount :type Integer))
  (bind _spawners (LocalVariables|GetSpawners))
  (for _index (range 0 (- PreviewAmount 1))
    (bind _outactors (Actor|GetAllActorsOfClass "/Game/Blueprints/BP_BowlingBallSpawner.BP_BowlingBallSpawner_C"))
    (for _array_element _outactors
      (if (Variables|/Game/Blueprints/BP_BowlingBallSpawner.BP_BowlingBallSpawner_C|GetbPreview _array_element)
        (Utilities|Array|RemoveItem _spawners _array_element)
        (else
          (Utilities|Array|AddUnique _spawners _array_element))))
    (bind _selectedball (CallFunction|FindWaveBall _index))
    (Default|SetPreview (.OutItem (Utilities|Array|Random (LocalVariables|GetSpawners))) _selectedball))
  (return))

(fn GivePlayerCurrency
  (bind _playerref (Variables|Default|GetPlayerRef))
  (bind _bpc_currencymanager (Variables|/Game/Blueprints/Player/BP_PlayerPawn.BP_PlayerPawn_C|GetBPC_CurrencyManager _playerref))
  (bind _outactors (Actor|GetAllActorsOfClass "/Game/Assets/BowlingPin/BP_BowlingPin.BP_BowlingPin_C"))
  (bind _output_get (Variables|PinScoring|SetPinsLeft (Utilities|Array|Length _outactors)))
  (Variables|/Game/Blueprints/Shop/BPC_CurrencyManager.BPC_CurrencyManager_C|SetPlayerCurrency _bpc_currencymanager (+ _output_get (Variables|/Game/Blueprints/Shop/BPC_CurrencyManager.BPC_CurrencyManager_C|GetPlayerCurrency _bpc_currencymanager)))
  (Default|UpdateCurrency (Variables|Default|GetShopRef)))