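; BPC_CurrencyManager is a shop Blueprint that tracks player currency and handles purchase attempts on props.
; The BuyingObject event stores the passed prop and, if valid, compares its Value against PlayerCurrency.
; An affordable prop has its cost deducted and sets CanBuy true; otherwise it prints "Not Enough Points" and sets CanBuy false.
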(event Custom|BuyingObject
  (params (PropRef :type BP%20Primary%20Data%20Shop%20Object%20Reference))
  (bind _output_get (Variables|Default|SetObjectData PropRef))
  (Utilities|IsValid _output_get
    (:Is%20Valid
      (if (<= (Variables|/Game/Blueprints/Shop/Data/BP_PrimaryDataShop.BP_PrimaryDataShop_C|GetValue _output_get) (Variables|Default|GetPlayerCurrency))
        (Variables|Default|SetPlayerCurrency (- (Variables|Default|GetPlayerCurrency) (Variables|/Game/Blueprints/Shop/Data/BP_PrimaryDataShop.BP_PrimaryDataShop_C|GetValue (Variables|Default|GetObjectData))))
        (Variables|Default|SetbCanBuy true)
        (else
          (Development|PrintString "Not Enough Points")
          (Variables|Default|SetbCanBuy false))))))