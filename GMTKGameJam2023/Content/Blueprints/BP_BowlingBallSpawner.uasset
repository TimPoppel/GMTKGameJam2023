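; Bowling ball spawner actor that previews an upcoming throw with an arrow, then spawns the ball aimed toward the pins.
; SetPreview stores the ball class, faces a randomly picked BP_PinSpawner and shows the arrow plane.
; The HasCurve map decides between a straight or curved arrow, with left or right chosen from the aim yaw.
; SpawnBall spawns the stored class along that direction and hides the preview.
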(event EventBeginPlay)

(event Collision|EventActorBeginOverlap
  (params (OtherActor :type Actor%20Object%20Reference)))

(event EventTick
  (params (DeltaSeconds :type Float%20%28single-precision%29)))

(fn ConstructionScript)

(fn SpawnBall
  (Game|SpawnActorfromClass (Variables|Default|GetBall%20to%20Spawn) (Math|Transform|MakeTransform (Transformation|GetActorLocation) (Variables|Default|GetShootDirection) "1.000000,1.000000,1.000000") "Undefined" "MultiplyWithRoot" 0 0)
  (CallFunction|RemovePreview)
  (return))

(fn SetPreview
  (params (BallToSpawn :type BP%20Bowling%20Ball%20Class%20Reference))
  (bind _plane (Variables|Default|GetPlane))
  (Variables|Default|SetBall%20to%20Spawn BallToSpawn)
  (bind _outactors (Actor|GetAllActorsOfClass "/Game/Blueprints/BP_PinSpawner.BP_PinSpawner_C"))
  (bind _output_get (Variables|Default|SetShootDirection (Math|Rotator|FindLookatRotation (Transformation|GetActorLocation) (Transformation|GetActorLocation (.OutItem (Utilities|Array|Random _outactors))))))
  (Transformation|SetWorldRotation (Variables|Default|GetDefaultSceneRoot) _output_get false false)
  (Rendering|Material|SetMaterial _plane 0 (Utilities|Select :Index (Math|Integer|SelectInt (Math|Integer|SelectInt 1 2 (> (.yaw (Variables|Default|GetShootDirection)) 9e+01)) 0 (.Value (Utilities|Map|Find (Variables|Default|GetHasCurve) (Variables|Default|GetBall%20to%20Spawn)))) :Option%200 "/Game/Art/Textures/M_ArrowForward.M_ArrowForward" :Option%201 "/Game/Art/Textures/M_ArrowLeft.M_ArrowLeft" :Option%202 "/Game/Art/Textures/M_ArrowRight.M_ArrowRight"))
  (Rendering|SetVisibility _plane true false)
  (Variables|Default|SetbPreview true)
  (return))

(fn RemovePreview
  (Rendering|SetVisibility (Variables|Default|GetPlane) false false)
  (Variables|Default|SetbPreview false)
  (return))