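; Bowling ball prop that launches itself along its forward vector with a random mesh, then reports to GM_Bowling when finished.
; BeginPlay dissolves it in via a material "Amount" timeline, then after a delay applies a mass-scaled impulse and optional curve spin based on yaw.
; Hits notify props and pins, with an empty SpecialEffect hook for props.
; A stillness or max-roll-time check ends the roll, fading and destroying the ball.
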(event OnComponentHit(Sphere1)
  (params (HitComponent :type Primitive%20Component%20Object%20Reference) (OtherActor :type Actor%20Object%20Reference) (OtherComp :type Primitive%20Component%20Object%20Reference) (NormalImpulse :type Vector :default "0, 0, 0") (Hit :type Hit%20Result%20Structure%20%28by%20ref%29))
  (Utilities|FlowControl|Sequence
    (:then_0
      (bind _asbp_prop_base (Utilities|Casting|CastToBP_PropBase OtherActor))
      (if (Variables|Default|GetBallCanSpecialEffect)
        (CallFunction|SpecialEffect _asbp_prop_base))
      (Default|GetHit _asbp_prop_base))
    (:then_1
      (bind _asbp_bowling_pin (Utilities|Casting|CastToBP_BowlingPin OtherActor))
      (Default|CallGetHit _asbp_bowling_pin))))

(event Custom|CheckIfBallStill
  (bind _sphere (Variables|Default|GetSphere))
  (bind _sourcematerial (Variables|Default|GetSourceMaterial))
  (if (Math|Float|NearlyEqual(Float) (Math|Vector|VectorLength (Transformation|GetComponentVelocity (Variables|Default|GetSphere1))) 0.0 3e+01)
    (bind _asgm_bowling (Utilities|Casting|CastToGM_Bowling (Game|GetGameMode) :!label _label))
    (Default|BallFinished _asgm_bowling)
    (bind _returnvalue (Rendering|Material|CreateDynamicMaterialInstance _sphere 0 _sourcematerial "None" :!class /Script/Engine.PrimitiveComponent))
    (bind _returnvalue_2 (Rendering|Material|CreateDynamicMaterialInstance _sphere 1 _sourcematerial "None" :!class /Script/Engine.PrimitiveComponent))
    (bind _newtrack_0 (Timeline|Timeline Play)
      (:Update
        (Rendering|Material|SetScalarParameterValue _returnvalue "Amount" _newtrack_0 :!class /Script/Engine.MaterialInstanceDynamic))
      (:Finished
        (Actor|DestroyActor)))
    (elif (> (Actor|GetGameTimeSinceCreation) (Variables|Default|GetMaxRollTime))
      (goto _label))))

(event Custom|Bowling%20Ball%20Reached%20end
  (bind _sphere (Variables|Default|GetSphere))
  (bind _sourcematerial (Variables|Default|GetSourceMaterial))
  (bind _asgm_bowling (Utilities|Casting|CastToGM_Bowling (Game|GetGameMode)))
  (Default|BallFinished _asgm_bowling)
  (bind _returnvalue (Rendering|Material|CreateDynamicMaterialInstance _sphere 0 _sourcematerial "None" :!class /Script/Engine.PrimitiveComponent))
  (bind _returnvalue_2 (Rendering|Material|CreateDynamicMaterialInstance _sphere 1 _sourcematerial "None" :!class /Script/Engine.PrimitiveComponent))
  (bind _newtrack_0 (Timeline|Timeline Play)
    (:Update
      (Rendering|Material|SetScalarParameterValue _returnvalue "Amount" _newtrack_0 :!class /Script/Engine.MaterialInstanceDynamic))
    (:Finished
      (Actor|DestroyActor))))

(event Custom|SpawnBallVisually
  (bind _sphere (Variables|Default|GetSphere))
  (bind _sourcematerial (Variables|Default|GetSourceMaterial))
  (bind _returnvalue (Rendering|Material|CreateDynamicMaterialInstance _sphere 0 _sourcematerial "None" :!class /Script/Engine.PrimitiveComponent))
  (bind _returnvalue_2 (Rendering|Material|CreateDynamicMaterialInstance _sphere 1 _sourcematerial "None" :!class /Script/Engine.PrimitiveComponent))
  (bind _newtrack_0 (Timeline|Timeline_0 ReverseFromEnd)
    (:Update
      (Rendering|Material|SetScalarParameterValue _returnvalue "Amount" _newtrack_0 :!class /Script/Engine.MaterialInstanceDynamic))))

(event Custom|Special%20Effect
  (params (Hit%20Actor :type BP%20Prop%20Base%20Object%20Reference)))

(event EventBeginPlay
  (bind _defaultsceneroot (Variables|Default|GetDefaultSceneRoot))
  (bind _returnvalue (Transformation|GetWorldRotation _defaultsceneroot))
  (Class|PrimitiveComponent|SetMassOverrideinKg (Variables|Default|GetSphere1) "None" (Variables|BallInfo|GetMass%20in%20Kg) true)
  (bind (_sphere _output) (CallFunction|SelectRandomStaticMesh))
  (Components|StaticMesh|SetStaticMesh _sphere _output)
  (CallFunction|SpawnBallVisually)
  (Variables|Default|SetLowAngle (Math|Float|InRange(Float) (.yaw _returnvalue) 88.0 92.0))
  (Variables|Default|SetEffectDirection (Math|Integer|SelectInt 1 -1 (> (.yaw _returnvalue) 9e+01)))
  (Utilities|FlowControl|Delay (Variables|Default|GetBallIdleTime))
  (Physics|AddImpulse (Variables|Default|GetSphere1) (* (* (Variables|BallInfo|GetMass%20in%20Kg) (Variables|BallInfo|GetImpulse%20speed)) (Transformation|GetActorForwardVector)) "None" false)
  (if (Variables|Default|GetBallCanSpin)
    (Class|PrimitiveComponent|SetAllPhysicsAngularVelocityinDegrees (Variables|Default|GetSphere1) (* (Math|Vector|MakeVector (* (Math|Float|SelectFloat (/ (* (Math|Random|RandomFloatinRange (Variables|Default|GetMinCurveSpeed) (Variables|Default|GetMaxCurveSpeed)) (Variables|Default|GetEffectDirection)) 2.0) (* (Math|Random|RandomFloatinRange (Variables|Default|GetMinCurveSpeed) (Variables|Default|GetMaxCurveSpeed)) (Variables|Default|GetEffectDirection)) (Variables|Default|GetLowAngle)) 1.0) (* (Math|Float|SelectFloat (/ (* (Math|Random|RandomFloatinRange (Variables|Default|GetMinCurveSpeed) (Variables|Default|GetMaxCurveSpeed)) (Variables|Default|GetEffectDirection)) 2.0) (* (Math|Random|RandomFloatinRange (Variables|Default|GetMinCurveSpeed) (Variables|Default|GetMaxCurveSpeed)) (Variables|Default|GetEffectDirection)) (Variables|Default|GetLowAngle)) 1.0) 0.0) (Transformation|GetActorForwardVector)) false))
  (Utilities|Time|SetTimerbyEvent (EventDispatchers|CreateEvent :!event Custom|CheckIfBallStill) 1.0 true))

(fn ConstructionScript)

(fn SelectRandomStaticMesh
  (bind _bowling_ball_1 (Variables|BowlingBallSkins|GetBowling%20Ball%201))
  (bind _bowling_ball_2 (Variables|BowlingBallSkins|GetBowling%20Ball%202))
  (bind _bowling_ball_3 (Variables|BowlingBallSkins|GetBowling%20Ball%203))
  (bind _bowling_ball_4 (Variables|BowlingBallSkins|GetBowling%20Ball%204))
  (bind _bowling_ball_5 (Variables|BowlingBallSkins|GetBowling%20Ball%205))
  (bind _array (Utilities|Array|MakeArray _bowling_ball_1 _bowling_ball_2 _bowling_ball_3 _bowling_ball_4 _bowling_ball_5))
  (return (Variables|Default|GetSphere) (Utilities|Array|Get(acopy) _array (Math|Random|RandomInteger (Utilities|Array|Length _array)))))