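; Base physical prop Blueprint with a mass and limited durability.
; BeginPlay overrides the Cube's mass with PropWeight.
; Each GetHit call plays a sound and decrements durability, destroying the actor after a short delay once it reaches the minimum.
; Cube overlaps with BP_PlayerPawn set the pawn's placement status to false on entry and back to true on exit.
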(event OnComponentBeginOverlap(Cube)
  (params (OverlappedComponent :type Primitive%20Component%20Object%20Reference) (OtherActor :type Actor%20Object%20Reference) (OtherComp :type Primitive%20Component%20Object%20Reference) (OtherBodyIndex :type Integer) (bFromSweep :type Boolean) (SweepResult :type Hit%20Result%20Structure%20%28by%20ref%29))
  (bind _asbp_player_pawn (Utilities|Casting|CastToBP_PlayerPawn OtherActor))
  (Default|UpdatePlacementStatus _asbp_player_pawn false))

(event OnComponentEndOverlap(Cube)
  (params (OverlappedComponent :type Primitive%20Component%20Object%20Reference) (OtherActor :type Actor%20Object%20Reference) (OtherComp :type Primitive%20Component%20Object%20Reference) (OtherBodyIndex :type Integer))
  (bind _asbp_player_pawn (Utilities|Casting|CastToBP_PlayerPawn OtherActor))
  (Default|UpdatePlacementStatus _asbp_player_pawn true))

(event Custom|GetHit
  (Audio|PlaySound2D (Variables|Audio|GetSound) 1.0 1.0 0.0 0 0)
  (bind _result (Math|Integer|DecrementInt (Variables|Default|GetPropDurability))
    (:%20%20
      (if (<= _result (Variables|Default|GetMinHealth))
        (Utilities|FlowControl|Delay (Variables|PropInfo|GetBreaking%20Delay))
        (Actor|DestroyActor)))))

(event EventBeginPlay
  (Class|PrimitiveComponent|SetMassOverrideinKg (Variables|Default|GetCube) "None" (Variables|PropInfo|GetPropWeight) true))

(event Collision|EventActorBeginOverlap
  (params (OtherActor :type Actor%20Object%20Reference)))

(event EventTick
  (params (DeltaSeconds :type Float%20%28single-precision%29)))

(fn ConstructionScript)