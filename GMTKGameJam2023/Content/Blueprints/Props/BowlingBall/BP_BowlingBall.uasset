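; A physics-driven bowling ball prop that launches itself forward and tells the bowling game mode when its roll is over.
; On BeginPlay it overrides its mass, picks one of five random meshes, applies a forward impulse after a short delay and starts a looping timer.
; Hits on prop actors trigger their GetHit.
; A near-zero velocity check or a reached-end event calls BallFinished on GM_Bowling and destroys the ball.
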(event OnComponentHit(Sphere1)
  (params (HitComponent :type Primitive%20Component%20Object%20Reference) (OtherActor :type Actor%20Object%20Reference) (OtherComp :type Primitive%20Component%20Object%20Reference) (NormalImpulse :type Vector :default "0, 0, 0") (Hit :type Hit%20Result%20Structure%20%28by%20ref%29))
  (if (== (Variables|Default|GetPropBase) (Utilities|GetClass OtherActor))
    (bind _asbp_prop_base (Utilities|Casting|CastToBP_PropBase OtherActor))
    (Default|GetHit _asbp_prop_base)))

(event Custom|CheckIfBallStill
  (if (Math|Float|NearlyEqual(Float) (Math|Vector|VectorLength (Transformation|GetComponentVelocity (Variables|Default|GetSphere1))) 0.0 3e+01)
    (bind _asgm_bowling (Utilities|Casting|CastToGM_Bowling (Game|GetGameMode)))
    (Default|BallFinished _asgm_bowling)
    (Actor|DestroyActor)
    (else
      (Development|PrintString "ball rolling fast"))))

(event Custom|Bowling%20Ball%20Reached%20end
  (bind _asgm_bowling (Utilities|Casting|CastToGM_Bowling (Game|GetGameMode)))
  (Default|BallFinished _asgm_bowling)
  (Actor|DestroyActor))

(event EventBeginPlay
  (Class|PrimitiveComponent|SetMassOverrideinKg (Variables|Default|GetSphere1) "None" (Variables|BallInfo|GetMass%20in%20Kg) true)
  (bind (_sphere _output) (CallFunction|SelectRandomStaticMesh))
  (Components|StaticMesh|SetStaticMesh _sphere _output)
  (Utilities|FlowControl|Delay 1.0)
  (Physics|AddImpulse (Variables|Default|GetSphere1) (* (Variables|BallInfo|GetImpulse%20speed) (Transformation|GetActorForwardVector)) "None" false)
  (Utilities|Time|SetTimerbyEvent (EventDispatchers|CreateEvent :!event Custom|CheckIfBallStill) 1.0 true))

(fn ConstructionScript)

(fn SelectRandomStaticMesh
  (bind _bowling_ball_1 (Variables|BowlingBallSkins|GetBowling%20Ball%201))
  (bind _bowling_ball_2 (Variables|BowlingBallSkins|GetBowling%20Ball%202))
  (bind _bowling_ball_3 (Variables|BowlingBallSkins|GetBowling%20Ball%203))
  (bind _bowling_ball_4 (Variables|BowlingBallSkins|GetBowling%20Ball%204))
  (bind _bowling_ball_5 (Variables|BowlingBallSkins|GetBowling%20Ball%205))
  (bind _array (Utilities|Array|MakeArray _bowling_ball_1 _bowling_ball_2 _bowling_ball_3 _bowling_ball_4 _bowling_ball_5))
  (return (Variables|Default|GetSphere) (Utilities|Array|Get(acopy) _array (Math|Random|RandomInteger (Utilities|Array|Length _array)))))