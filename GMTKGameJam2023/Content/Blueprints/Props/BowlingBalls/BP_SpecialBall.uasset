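; BP_SpecialBall is a bowling ball prop that sets off a one-time radial impulse through its SpecialEffect event.
; The hit actor's PropWeight selects a small, medium or big explosion strength, which is multiplied by that weight to set the RadialForce impulse.
; A FirstHitDone flag limits the impulse to the first hit, and the resulting strength is printed as debug output.
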(event EventSpecialEffect
  (params (Hit%20Actor :type BP%20Prop%20Base%20Object%20Reference))
  (if (>= (Variables|/Game/Blueprints/Props/BP_PropBase.BP_PropBase_C|GetPropWeight Hit%20Actor) 1e+01)
    (if (>= (Variables|/Game/Blueprints/Props/BP_PropBase.BP_PropBase_C|GetPropWeight Hit%20Actor) 2e+01)
      (Variables|Default|SetExplosion%20Strength (Variables|Default|GetBigExplosion))
      (else
        (Variables|Default|SetExplosion%20Strength (Variables|Default|GetMediumExplosion))))
    (else
      (Variables|Default|SetExplosion%20Strength (Variables|Default|GetSmallExplosion))))
  (if (not (Variables|Default|GetFirstHitDone))
    (Variables|Default|SetFirstHitDone true)
    (Variables|/Script/Engine.RadialForceComponent|SetImpulseStrength (Variables|Default|GetRadialForce) (* (Variables|/Game/Blueprints/Props/BP_PropBase.BP_PropBase_C|GetPropWeight Hit%20Actor) (Variables|Default|GetExplosion%20Strength)))
    (Development|PrintString (Utilities|String|ToString(Float) (* (Variables|/Game/Blueprints/Props/BP_PropBase.BP_PropBase_C|GetPropWeight Hit%20Actor) (Variables|Default|GetExplosion%20Strength))))
    (Class|RadialForceComponent|FireImpulse (Variables|Default|GetRadialForce))))

(fn ConstructionScript
  (|CallParentFunction))