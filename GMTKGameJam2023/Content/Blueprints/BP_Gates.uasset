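; BP_Gates is a gate actor that slides from its placed position to a target position when PutupGates is called.
; PutupGates passes through a DoOnce, then records the actor location and the world location of the EndLocation component as start and end points.
; A Timeline's Alpha drives a vector lerp that sets the actor location each update, without sweeping.
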(event Custom|Put%20up%20Gates
  (Utilities|FlowControl|DoOnce false
    (:Completed
      (Variables|Default|SetStartPosition (Transformation|GetActorLocation))
      (Variables|Default|SetEndPosition (Transformation|GetWorldLocation (Variables|Default|GetEndLocation)))
      (bind _alpha (Timeline|Timeline Play)
        (:Update
          (Transformation|SetActorLocation (Math|Vector|Lerp(Vector) (Variables|Default|GetStartPosition) (Variables|Default|GetEndPosition) _alpha) false false))))))

(event Collision|EventActorBeginOverlap
  (params (OtherActor :type Actor%20Object%20Reference)))

(event EventTick
  (params (DeltaSeconds :type Float%20%28single-precision%29)))

(fn ConstructionScript)