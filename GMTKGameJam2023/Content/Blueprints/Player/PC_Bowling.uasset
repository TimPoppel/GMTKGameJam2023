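; PC_Bowling is a player controller that lets the player position, rotate and spawn props with the mouse through BP_PlayerPawn.
; Each tick it traces the Visibility channel from the deprojected cursor, ignoring the pawn, and moves the pawn to the hit location.
; The mouse wheel yaws the pawn at a configurable speed, and a left click calls SpawnProp on it.
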(event EventBeginPlay
  (bind _asbp_player_pawn (Utilities|Casting|CastToBP_PlayerPawn (Game|Player|GetPlayerPawn 0)))
  (Variables|Default|SetPlayerRef _asbp_player_pawn))

(event EventTick
  (params (DeltaSeconds :type Float%20%28single-precision%29))
  (bind (_worldlocation _worlddirection) (Game|Player|ConvertMouseLocationToWorldSpace))
  (bind _outhit (Collision|LineTraceByChannel _worldlocation (+ _worldlocation (* _worlddirection (Variables|Default|GetLineTraceDepth))) "TraceTypeQuery1" false (Utilities|Array|MakeArray (Variables|Default|GetPlayerRef)) "None" true "(R=1.000000,G=0.000000,B=0.000000,A=1.000000)" "(R=0.000000,G=1.000000,B=0.000000,A=1.000000)" 1.0))
  (Variables|Default|SetLineTraceLocation (.Location (Collision|BreakHitResult _outhit)))
  (Transformation|SetActorLocation (Variables|Default|GetPlayerRef) (.Location (Collision|BreakHitResult _outhit)) false false))

(event Input|MouseEvents|MouseWheelAxis
  (params (AxisValue :type Float%20%28single-precision%29))
  (Class|Actor|AddActorWorldRotation (Variables|Default|GetPlayerRef) (Math|Rotator|MakeRotator 0.0 0.0 (* AxisValue (Variables|Default|GetPropRotationSpeed)))))

(event Input|MouseEvents|LeftMouseButton
  (params (Key :type Key%20Structure :default "None"))
  (:Pressed
    (Default|SpawnProp (Variables|Default|GetPlayerRef))))

(fn ConstructionScript)