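; Player pawn for a bowling game's build phase, previewing and placing props bought from the shop.
; A shop-bound event passes prop data that sets the preview mesh's shape, scale and rotation.
; Placement status swaps good/bad materials using build-zone, prop and no-build-zone overlaps, though failed overlap checks leave the previous state unchanged.
; SpawnProp requires valid placement, build phase and selection, buys through BPCCurrencyManager, spawns the actor, then notifies the shop.
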(event Custom|ChangeProp
  (params (PropData :type BP%20Primary%20Data%20Shop%20Object%20Reference))
  ;[1 1 1] Update prob
  (Variables|Default|SetProp%20Data PropData)
  (CallFunction|ChangePropType (Variables|/Game/Blueprints/Shop/Data/BP_PrimaryDataShop.BP_PrimaryDataShop_C|GetActorClass PropData) (Variables|/Game/Blueprints/Shop/Data/BP_PrimaryDataShop.BP_PrimaryDataShop_C|GetScale PropData) (Variables|/Game/Blueprints/Shop/Data/BP_PrimaryDataShop.BP_PrimaryDataShop_C|GetMesh PropData) (Variables|/Game/Blueprints/Shop/Data/BP_PrimaryDataShop.BP_PrimaryDataShop_C|GetRotation PropData))
  (CallFunction|ToggleVisibility true))

(event EventBeginPlay
  (Variables|/Game/Blueprints/Shop/BPC_CurrencyManager.BPC_CurrencyManager_C|SetPlayerCurrency (Variables|Default|GetBPC_CurrencyManager) (Variables|Default|GetPlayerStartingMoney))
  (bind _asgm_bowling (Utilities|Casting|CastToGM_Bowling (Game|GetGameMode)))
  (bind _output_get (Variables|Default|SetGamemodeRef _asgm_bowling))
  (EventDispatchers|BindEventtoSelectedObject (Variables|/Game/Blueprints/GM_Bowling.GM_Bowling_C|GetShopRef _output_get) (EventDispatchers|CreateEvent :!event Custom|ChangeProp))
  (CallFunction|ToggleVisibility false))

(fn ConstructionScript)

(fn UpdatePlacementStatus
  (params (IsValidPlacement :type Boolean))
  (if IsValidPlacement
    (if (Math|Boolean|ANDBoolean (> (Utilities|Array|Length (Collision|GetOverlappingActors "/Game/Blueprints/Player/BP_BuildZone.BP_BuildZone_C" :!class /Script/Engine.Actor)) 0) (<= (Utilities|Array|Length (Collision|GetOverlappingActors "/Game/Blueprints/Props/BP_PropBase.BP_PropBase_C" :!class /Script/Engine.Actor)) 0) (<= (Utilities|Array|Length (Collision|GetOverlappingActors "/Game/Blueprints/Player/BP_NoBuildZone.BP_NoBuildZone_C" :!class /Script/Engine.Actor)) 0))
      (Rendering|Material|SetMaterial (Variables|Default|GetStaticMesh) 0 "/Game/Art/Materials/M_PlacementGood.M_PlacementGood")
      (else
        (return)))
    (else
      (Rendering|Material|SetMaterial (Variables|Default|GetStaticMesh) 0 "/Game/Art/Materials/M_PlacementBad.M_PlacementBad")))
  (Variables|Default|SetbValidPlacement IsValidPlacement)
  (return))

(fn SpawnProp
  (bind _bvalidplacement (Variables|Default|GetbValidPlacement))
  (bind _buildingphaseenabled (Variables|Default|GetBuildingPhaseEnabled))
  (bind _bpropselected (Variables|Default|GetbPropSelected))
  (bind _bpc_currencymanager (Variables|Default|GetBPC_CurrencyManager))
  (bind _returnvalue (Math|Boolean|ANDBoolean _bvalidplacement _buildingphaseenabled _bpropselected))
  (if _returnvalue
    (Default|BuyingObject _bpc_currencymanager (Variables|Default|GetProp%20Data))
    (if (and _returnvalue (Variables|/Game/Blueprints/Shop/BPC_CurrencyManager.BPC_CurrencyManager_C|GetbCanBuy _bpc_currencymanager))
      (Game|SpawnActorfromClass (Variables|Default|GetSelectedPropClass) (Math|Transform|MakeTransform (+ (Transformation|GetActorLocation) (Math|Vector|MakeVector 0.0 0.0 (Variables|Default|GetSpawnPropHeight))) (Transformation|GetActorRotation) (Variables|Default|GetSelectedPropScale)) "Undefined" "MultiplyWithRoot" 0 0)
      (Default|CallPlayerBoughtItem (Variables|/Game/Blueprints/GM_Bowling.GM_Bowling_C|GetShopRef (Variables|Default|GetGamemodeRef)))
      (return true)
      (else
        _)))
  (return false))

(fn ChangePropType
  (params (PropClass :type BP%20Prop%20Base%20Class%20Reference) (Scale :type Vector) (PropMesh :type Static%20Mesh%20Object%20Reference) (Rotation :type Rotator))
  (Variables|Default|SetSelectedPropClass PropClass)
  (Variables|Default|SetSelectedPropScale Scale)
  (Variables|Default|SetStartRotationProp Rotation)
  (Components|StaticMesh|SetStaticMesh (Variables|Default|GetStaticMesh) PropMesh)
  (Transformation|SetWorldScale3D (Variables|Default|GetStaticMesh) (Variables|Default|GetSelectedPropScale))
  (Transformation|SetRelativeRotation (Variables|Default|GetStaticMesh) (Variables|Default|GetStartRotationProp) false false)
  (return))

(fn ToggleVisibility
  (params (bVisibile :type Boolean))
  (Rendering|SetVisibility (Variables|Default|GetStaticMesh) bVisibile false)
  (Variables|Default|SetbPropSelected bVisibile)
  (return))